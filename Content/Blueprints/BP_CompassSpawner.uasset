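; BP_CompassSpawner is an actor that is visible only while no BP_Compass exists in the level; it contains no spawning logic itself.
; Every Tick, it sets the Cube's world rotation to the CompassSpawner component's roll and pitch with a fixed world yaw.
; It also polls GetAllActorsOfClass each frame and hides or shows the whole actor based on whether any compass is found.
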(event `self.ReceiveTick`
  (params (DeltaSeconds :type "Float (single-precision)"))
  (`SceneComponent.K2_SetWorldRotation` (`self.Cube`) (`KismetMathLibrary.MakeRotator` (.roll (`SceneComponent.K2_GetComponentRotation` (`self.CompassSpawner`))) (.pitch (`SceneComponent.K2_GetComponentRotation` (`self.CompassSpawner`))) 180.0) false false)
  (bind _outactors (`GameplayStatics.GetAllActorsOfClass` "/Game/Blueprints/BP_Compass.BP_Compass_C"))
  (if (<= (`KismetArrayLibrary.Array_Length` _outactors) 0)
    (`self.SetActorHiddenInGame` false)
    (else
      (`self.SetActorHiddenInGame` true))))

(fn `UserConstructionScript`)