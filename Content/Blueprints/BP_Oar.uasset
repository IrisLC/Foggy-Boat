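; BP_Oar is a grabbable oar that paddles BP_Boat while held in the water.
; Grab events on the handle and head track holding, and Box overlaps set the in-water flag.
; Each tick, a held, submerged oar passes its collider and location to the boat's Paddling and plays a sound.
; An unheld oar destroys itself after a three-second delay; the ReturnPostion call that would reattach it is disconnected.
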(event `self.ReceiveBeginPlay`
  (`self.SetUp`))

(event `self.ReceiveTick`
  (params (DeltaSeconds :type "Float (single-precision)"))
  (bind _returnvalue (`self.K2_GetActorLocation`))
  (bind _box (`self.Box`))
  (if (or (`self.Grabbed Head`) (`self.Grabbed Handle`))
    (set `self.OriginalPos` false)
    (if (`self.isInWater`)
      ; Rowing
      (`PrimitiveComponent.GetPhysicsLinearVelocity` _box "None")
      (bind _returnvalue_2 (`GameplayStatics.GetActorOfClass` "/Game/Blueprints/BP_Boat.BP_Boat_C"))
      (`/Game/Blueprints/BP_Boat.Paddling` _returnvalue_2 _box _returnvalue)
      (`GameplayStatics.PlaySoundAtLocation` "/Game/Assets/Sounds/OarSound_Cue.OarSound_Cue" _returnvalue (struct) 1.0 1.0 0.0 null null null null))
    (else
      ; Returns the Paddle to the Boat
      (bind _returnvalue_3 (`GameplayStatics.GetActorOfClass` "/Game/Blueprints/BP_BoatHolder.BP_BoatHolder_C"))
      (bind _returnvalue_4 (`GameplayStatics.GetActorOfClass` "/Game/Blueprints/BP_Boat.BP_Boat_C"))
      (`KismetSystemLibrary.Delay` 3.0)
      (`self.K2_DestroyActor`))))

(event `self.Box.OnComponentBeginOverlap`
  (params (OverlappedComponent :type "PrimitiveComponent Object Reference") (OtherActor :type "Actor Object Reference") (OtherComp :type "PrimitiveComponent Object Reference") (OtherBodyIndex :type Integer) (bFromSweep :type Boolean) (SweepResult :type "HitResult Structure (by ref)"))
  (set `self.isInWater` true))

(event `self.Box.OnComponentEndOverlap`
  (params (OverlappedComponent :type "PrimitiveComponent Object Reference") (OtherActor :type "Actor Object Reference") (OtherComp :type "PrimitiveComponent Object Reference") (OtherBodyIndex :type Integer))
  (set `self.isInWater` false))

(event `self.GrabHandle.OnGrabbed`
  (set `self.Grabbed Handle` true))

(event `self.GrabHandle.OnDropped`
  (set `self.Grabbed Handle` false)
  (`PrimitiveComponent.SetSimulatePhysics` (`self.oar1`) true))

(event `self.GrabHead.OnGrabbed`
  (set `self.Grabbed Head` true))

(event `self.GrabHead.OnDropped`
  (set `self.Grabbed Head` false)
  (`PrimitiveComponent.SetSimulatePhysics` (`self.oar1`) true)
  (set `self.OriginalPos` true))

(fn `ReturnPostion`
  (params (Boat :type "/Game/Blueprints/BP_Boat Object Reference") (`Boat Holder` :type "/Game/Blueprints/BP_BoatHolder Object Reference"))
  (bind _oar1 (`self.oar1`))
  (bind _returnvalue (>= (`KismetMathLibrary.Vector_Distance` (`self.K2_GetActorLocation` `Boat Holder`) (`self.K2_GetActorLocation`)) 400.0))
  (if (or _returnvalue (and _returnvalue (`self.isInWater`)))
    (`/Game/XRFramework/Blueprints/BP_GrabComponent.OnDropped` (`self.GrabHandle`))
    (`/Game/XRFramework/Blueprints/BP_GrabComponent.OnDropped` (`self.GrabHead`))
    (`PrimitiveComponent.SetSimulatePhysics` _oar1 false)
    (`SceneComponent.K2_SetRelativeLocationAndRotation` _oar1 (+ (`self.K2_GetActorLocation` Boat) (`self.Original Pos`)) (`self.Original Rot`) false false)))

(fn `SetUp`
  (set `self.isInWater` false)
  (set `self.OriginalPos` false))

(fn `UserConstructionScript`)