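; BP_OarSpawner is an actor with an oar component and grab points on head and handle, available only while no BP_Oar exists in the world.
; Every Tick it searches for BP_Oar actors, then toggles its visibility, both GrabType settings and the Oar1 component's tick to match.
; The graph spawns nothing itself and prints a debug message on each update.
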(event `self.ReceiveTick`
  (params (DeltaSeconds :type "Float (single-precision)"))
  (bind _oar1 (`self.oar1`))
  (bind _outactors (`GameplayStatics.GetAllActorsOfClass` "/Game/Blueprints/BP_Oar.BP_Oar_C"))
  (if (<= (`KismetArrayLibrary.Array_Length` _outactors) 0)
    (set `/Game/XRFramework/Blueprints/BP_GrabComponent.GrabType` "NewEnumerator4" (`self.GrabHead`))
    (set `/Game/XRFramework/Blueprints/BP_GrabComponent.GrabType` "NewEnumerator4" (`self.GrabHandle`))
    (`self.SetActorHiddenInGame` false)
    (`KismetSystemLibrary.PrintText` "showing")
    (`ActorComponent.SetComponentTickEnabled` _oar1 true)
    (else
      (set `/Game/XRFramework/Blueprints/BP_GrabComponent.GrabType` "NewEnumerator0" (`self.GrabHead`))
      (set `/Game/XRFramework/Blueprints/BP_GrabComponent.GrabType` "NewEnumerator0" (`self.GrabHandle`))
      (`self.SetActorHiddenInGame` true)
      (`KismetSystemLibrary.PrintText` "Hiding")
      (`ActorComponent.SetComponentTickEnabled` _oar1 false))))

(fn `UserConstructionScript`)