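; Boat Blueprint that turns oar movement into propulsion and steering through a Paddling function, which nothing in this file calls.
; Paddling reads an oar collider's physics velocity and, past thresholds, applies a scaled, inverted force to the boat mesh in local space.
; It also calls MovingRotation, which rotates the boat by a small fixed step, choosing direction by dotting the oar-to-boat vector with the mesh's forward vector.
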(event `self.ReceiveBeginPlay`)

(event `self.ReceiveTick`
  (params (DeltaSeconds :type "Float (single-precision)")))

(fn `MovingRotation`
  (params (`Oar Collider` :type "BoxComponent Object Reference") (OarLocation :type "Vector Structure"))
  (bind _staticmesh (`self.StaticMesh`))
  (bind _returnvalue (`PrimitiveComponent.GetPhysicsLinearVelocity` `Oar Collider` "None"))
  (bind _x (.x _returnvalue))
  (bind _y (.y _returnvalue))
  (if (and (or (> _x 2.0) (< _x -2.0)) (or (> _y 2.0) (< _y -2.0)))
    (if (> (`KismetMathLibrary.Dot_VectorVector` (`KismetMathLibrary.Normal` (- (`SceneComponent.K2_GetComponentLocation` _staticmesh) OarLocation)) (`SceneComponent.GetForwardVector` _staticmesh)) 0.0)
      (`self.K2_AddActorLocalRotation` (struct :`Pitch` 0.1) true)
      (else
        (`self.K2_AddActorLocalRotation` (struct :`Pitch` -0.1) true)))))

(fn `Paddling`
  (params (`Box Collider` :type "BoxComponent Object Reference") (OarLocation :type "Vector Structure"))
  (`self.MovingRotation` `Box Collider` OarLocation)
  (bind _returnvalue (`PrimitiveComponent.GetPhysicsLinearVelocity` `Box Collider` "None"))
  (bind _x (.x _returnvalue))
  (bind _z (.z _returnvalue))
  (if (and (or (> _x 0.0) (< _x 0.0)) (or (> _z 3.0) (< _z -3.0)))
    (`PrimitiveComponent.AddForceAtLocationLocal` (`self.StaticMesh`) (* (`KismetMathLibrary.InverseTransformDirection` (`self.GetTransform`) _returnvalue) (-0.25 0.0 -2.0)) (0.0 0.0 0.0) "None")))

(fn `UserConstructionScript`)